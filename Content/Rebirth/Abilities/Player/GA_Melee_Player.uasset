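; GA_Melee_Player is a player gameplay ability for melee attacks that chains montage sections.
; On activation it commits, then looks up the montage's currently playing section in SectionMap to choose the start section, falling back to None when unmapped.
; It plays the montage with an event-listening task, applying effect containers for received gameplay event tags, and ends on blend out, interruption or cancellation.
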(event `self.K2_ActivateAbility`
  (bind (_value _returnvalue) (`BlueprintMapLibrary.Map_Find` (`self.SectionMap`) (`AnimInstance.Montage_GetCurrentSection` (`SkeletalMeshComponent.GetAnimInstance` (`self.GetOwningComponentFromActorInfo`)) (`self.MontageToPlay`))))
  (bind _returnvalue_2 (`self.K2_CommitAbility`))
  (if _returnvalue_2
    (if _returnvalue
      (set `self.TargetSection` _value)
      (else
        (set `self.TargetSection` "None")))
    (bind (_asynctaskproxy _eventtag _eventdata) (`PlayMontageAndWaitForEvent.PlayMontageAndWaitForEvent` "None" (`self.MontageToPlay`) (struct) 1.0 (`self.TargetSection`))
      (:`OnBlendOut`
        (`self.K2_EndAbility` :!label _label))
      (:`OnInterrupted`
        (goto _label))
      (:`OnCancelled`
        (goto _label))
      (:`EventReceived`
        (`self.ApplyEffectContainer` _eventtag _eventdata)))))