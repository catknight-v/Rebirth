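; Anim notify state that marks the active hit window of the player's melee weapon during attack animations.
; On begin, it casts the mesh owner to BP_RebirthCombatPC and, if the melee weapon is on, calls BeginWeaponAttack on its MeleeWeaponActor with the Event.Melee tag.
; On end, it repeats the same checks and calls EndWeaponAttack to close the window.
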(fn `Received_NotifyBegin`
  (params (MeshComp :type "SkeletalMeshComponent Object Reference") (Animation :type "AnimSequenceBase Object Reference") (TotalDuration :type "Float (double-precision)"))
  (returns (ReturnValue :type Boolean))
  (bind _asbp_rebirth_combat_pc (cast `/Game/Rebirth/Blueprints/Characters/BP_RebirthCombatPC` (`ActorComponent.GetOwner` MeshComp)))
  (bind _returnvalue (`RebirthCombatPC.IsMeleeWeaponOn` _asbp_rebirth_combat_pc))
  (if _returnvalue
    (bind _asmelee_weapon_actor (cast `MeleeWeaponActor` (`RebirthCombatPC.MeleeWeapon` _asbp_rebirth_combat_pc)))
    (`MeleeWeaponActor.BeginWeaponAttack` _asmelee_weapon_actor (struct :`TagName` "Event.Melee"))
    (return false)))

(fn `Received_NotifyEnd`
  (params (MeshComp :type "SkeletalMeshComponent Object Reference") (Animation :type "AnimSequenceBase Object Reference"))
  (returns (ReturnValue :type Boolean))
  (bind _asbp_rebirth_combat_pc (cast `/Game/Rebirth/Blueprints/Characters/BP_RebirthCombatPC` (`ActorComponent.GetOwner` MeshComp)))
  (bind _returnvalue (`RebirthCombatPC.IsMeleeWeaponOn` _asbp_rebirth_combat_pc))
  (if _returnvalue
    (bind _asmelee_weapon_actor (cast `MeleeWeaponActor` (`RebirthCombatPC.MeleeWeapon` _asbp_rebirth_combat_pc)))
    (`MeleeWeaponActor.EndWeaponAttack` _asmelee_weapon_actor)
    (return false)))