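; Anim notify state that marks the window in an animation during which the Lost Goust's talon weapon performs a melee attack.
; On begin, it casts the mesh owner to BP_LostGoust and calls BeginWeaponAttack on WeaponTalon with the Event.Melee tag.
; On end, it calls EndWeaponAttack on the same weapon, and both handlers do nothing for other owner types.
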(fn `Received_NotifyBegin`
  (params (MeshComp :type "SkeletalMeshComponent Object Reference") (Animation :type "AnimSequenceBase Object Reference") (TotalDuration :type "Float (double-precision)"))
  (returns (ReturnValue :type Boolean))
  (bind _asbp_lost_goust (cast `/Game/Rebirth/Blueprints/Characters/BP_LostGoust` (`ActorComponent.GetOwner` MeshComp)))
  (`MeleeWeaponActor.BeginWeaponAttack` (`/Game/Rebirth/Blueprints/Characters/BP_LostGoust.WeaponTalon` _asbp_lost_goust) (struct :`TagName` "Event.Melee"))
  (return false))

(fn `Received_NotifyEnd`
  (params (MeshComp :type "SkeletalMeshComponent Object Reference") (Animation :type "AnimSequenceBase Object Reference"))
  (returns (ReturnValue :type Boolean))
  (bind _asbp_lost_goust (cast `/Game/Rebirth/Blueprints/Characters/BP_LostGoust` (`ActorComponent.GetOwner` MeshComp)))
  (`MeleeWeaponActor.EndWeaponAttack` (`/Game/Rebirth/Blueprints/Characters/BP_LostGoust.WeaponTalon` _asbp_lost_goust))
  (return false))