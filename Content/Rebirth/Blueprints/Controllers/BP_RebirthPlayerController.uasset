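; Player controller for Rebirth that handles streamed level loading and level resets behind a fading overlay widget.
; On begin play it reads the level name and start location from the current save game, streams the level in and moves the player there.
; LevelReset fades in and reloads the level, then PushForwardLevel, blocked during the reload, resets combat, returns the player to the start and restores Free mode.
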(event `self.ReceiveBeginPlay`
  (bind _levelresetwidget (`self.LevelResetWidget`))
  (bind _asbp_rebirth_game_instance (cast `/Game/Rebirth/Blueprints/Rebirth/BP_RebirthGameInstance` (`GameplayStatics.GetGameInstance`)))
  (bind _returnvalue (`RebirthGameInstance.GetCurrentSaveGame` _asbp_rebirth_game_instance))
  (bind _returnvalue_2 (`RebirthSaveGame.GetCurrentLevelName` _returnvalue))
  (set `self.CurrentLevelName` _returnvalue_2)
  (bind _returnvalue_3 (`RebirthSaveGame.GetCurrentLevelStart` _returnvalue))
  (set `self.CurrentLevelStart` _returnvalue_3)
  (bind _returnvalue_4 (`|CreateWidget` "/Game/Rebirth/UI/BP_LevelResetUserWidget.BP_LevelResetUserWidget_C"))
  (bind _output_get (set `self.LevelResetWidget` _returnvalue_4))
  (`UserWidget.AddToViewport` _output_get 0)
  (`Widget.SetRenderOpacity` _levelresetwidget 1.0)
  (`GameplayStatics.LoadStreamLevel` (`self.CurrentLevelName`) true)
  (`self.K2_SetActorLocation` (`GameplayStatics.GetPlayerCharacter` 0) (`self.CurrentLevelStart`) false false)
  (`KismetSystemLibrary.Delay` 1.0)
  (`/Game/Rebirth/UI/BP_LevelResetUserWidget.FadeOut` _levelresetwidget))

(event `LevelReset`
  (bind _currentlevelname (`self.CurrentLevelName`))
  (`KismetSystemLibrary.Delay` 2.0)
  (`/Game/Rebirth/UI/BP_LevelResetUserWidget.FadeIn` (`self.LevelResetWidget`))
  (set `self.bLevelReset` true)
  (`KismetSystemLibrary.Delay` 1.0)
  (bind _asbp_rebirth_game_instance (cast `/Game/Rebirth/Blueprints/Rebirth/BP_RebirthGameInstance` (`GameplayStatics.GetGameInstance`)))
  (bind _returnvalue (`RebirthGameInstance.GetCurrentSaveGame` _asbp_rebirth_game_instance))
  (bind _returnvalue_2 (`RebirthSaveGame.GetCurrentLevelName` _returnvalue))
  (set `self.CurrentLevelName` _returnvalue_2)
  (bind _returnvalue_3 (`RebirthSaveGame.GetCurrentLevelStart` _returnvalue))
  (set `self.CurrentLevelStart` _returnvalue_3)
  (`GameplayStatics.UnloadStreamLevel` _currentlevelname)
  (`GameplayStatics.LoadStreamLevel` _currentlevelname true)
  (set `self.bLevelReset` false)
  (`/Game/Rebirth/UI/BP_LevelResetUserWidget.EBlink` (`self.LevelResetWidget`))
  (`self.SetGameMode` "Level"))

(event `self.PushForwardLevel`
  (bind _returnvalue (`GameplayStatics.GetPlayerCharacter` 0))
  (if (not (`self.bLevelReset`))
    (bind _asrebirth_combat_character_base (cast `RebirthCombatCharacterBase` _returnvalue))
    (`RebirthCombatCharacterBase.CombatReset` _asrebirth_combat_character_base)
    (`self.K2_SetActorLocation` _returnvalue (`self.CurrentLevelStart`) false false)
    (`/Game/Rebirth/UI/BP_LevelResetUserWidget.FadeOut` (`self.LevelResetWidget`))
    (`self.SetGameMode` "Free")))

(fn `UserConstructionScript`)