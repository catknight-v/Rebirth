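; BP_MeleeWeaponBase is a base melee weapon Blueprint meant to report hits to its instigator through Gameplay Ability System events.
; A DoOnce gates an AttackEventTag event carrying instigator and overlapped actor, and resets shortly after overlap ends.
; The gate's entry, which checks Attacking and a differing actor class, is disconnected and BeginOverlap is empty, so no event is sent.
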(event `self.ReceiveActorBeginOverlap`
  (params (OtherActor :type "Actor Object Reference")))

(event `self.ReceiveActorEndOverlap`
  (params (OtherActor :type "Actor Object Reference"))
  (bind _returnvalue (`self.GetInstigator`))
  (`KismetSystemLibrary.Delay` 0.2)
  (`/Engine/EditorBlueprintResources/StandardMacros.DoOnce` false :!via `Reset`
    (:`Completed`
      (`AbilitySystemBlueprintLibrary.SendGameplayEventToActor` _returnvalue (`self.AttackEventTag`) (make `GameplayEventData` (struct) _returnvalue (stale `self.ReceiveActorBeginOverlap` OtherActor))))))

(fn `UserConstructionScript`)