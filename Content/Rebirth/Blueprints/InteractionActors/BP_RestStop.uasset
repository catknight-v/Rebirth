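; BP_RestStop is an interactable rest point actor.
; Entering or leaving its interactable area fades its EWidget in or out.
; Interacting has the Rebirth player controller play the rest act, then after a short delay calls ActivateInitAbilities on the interacting combat character.
; Its CanInteract function always returns false.
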(event `InteractionInterface.EnterInteractableArea`
  (params (Interactor :type "Actor Object Reference"))
  (bind _asbp_ewidget (cast `/Game/Rebirth/UI/BP_EWidget` (`WidgetComponent.GetUserWidgetObject` (`self.EWidget`))))
  (`/Game/Rebirth/UI/BP_EWidget.EFadeIn` _asbp_ewidget))

(event `InteractionInterface.LeaveInteractableArea`
  (params (Interactor :type "Actor Object Reference"))
  (bind _asbp_ewidget (cast `/Game/Rebirth/UI/BP_EWidget` (`WidgetComponent.GetUserWidgetObject` (`self.EWidget`))))
  (`/Game/Rebirth/UI/BP_EWidget.EFadeOut` _asbp_ewidget))

(event `InteractionInterface.InteractWith`
  (params (Interactor :type "Actor Object Reference"))
  (bind _asrebirth_player_controller (cast `RebirthPlayerController` (`GameplayStatics.GetPlayerController` 0)))
  (`RebirthPlayerController.PlayAnAct` _asrebirth_player_controller "/Game/Rebirth/Acts/Act_Rest.Act_Rest_C")
  (`KismetSystemLibrary.Delay` 2.5)
  (bind _asrebirth_combat_character_base (cast `RebirthCombatCharacterBase` Interactor))
  (`RebirthCombatCharacterBase.ActivateInitAbilities` _asrebirth_combat_character_base))

(fn `CanInteract`
  (params (Interactor :type "Actor Object Reference"))
  (returns (ReturnValue :type Boolean))
  (return false))

(fn `UserConstructionScript`)