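; BP_ActTrack is an actor that moves its owner along a timed vertical track, starting from the owner's location at BeginPlay.
; Each Tick sets a cosine-eased Z offset, scaled by Distance, until the track actor's age reaches Duration.
; At half Duration the offset flips sign, so the owner rises, snaps below its start, then rises back toward it.
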(event `self.ReceiveBeginPlay`
  (bind _output_get (set `self.MoveActor` (`self.GetOwner`)))
  (set `self.PreLoction` (`self.K2_GetActorLocation` _output_get)))

(event `self.ReceiveTick`
  (params (DeltaSeconds :type "Float (single-precision)"))
  (bind _returnvalue (`self.GetGameTimeSinceCreation`))
  (bind _duration (`self.Duration`))
  (if (not (>= _returnvalue _duration))
    (if (>= _returnvalue (/ _duration 2.0))
      (set `self.Plus` -1.0)
      (else
        (set `self.Plus` 1.0)))
    (`self.K2_SetActorLocation` (`self.MoveActor`) (+ (`KismetMathLibrary.MakeVector` 0.0 0.0 (* (+ (- 0.0 (`KismetMathLibrary.DegCos` (/ (* _returnvalue 180.0) (`self.Duration`)))) (`self.Plus`)) (`self.Distance`))) (`self.PreLoction`)) false false)))

(fn `UserConstructionScript`)