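; SMFadeAnim is a short-lived helper actor that fades a scalar parameter on a dynamic material instance in or out.
; Init stores the material and fade direction, then Tick steps the ValName parameter up or down by FadeSpeed scaled by delta time.
; It destroys itself once the value reaches 0 or 1 in that direction, or after half a second has passed since creation.
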(event `Init`
  (params (MaterialInstanceDynamic :type "MaterialInstanceDynamic Object Reference") (FadeIn :type Boolean))
  (set `self.MaterialInstanceDynamic` MaterialInstanceDynamic)
  (set `self.FadeIn` FadeIn))

(event `self.ReceiveTick`
  (params (DeltaSeconds :type "Float (single-precision)"))
  (bind _fadein (`self.FadeIn`))
  (bind _materialinstancedynamic (`self.MaterialInstanceDynamic`))
  (bind _valname (`self.ValName`))
  (bind _returnvalue (* DeltaSeconds (`self.FadeSpeed`)))
  (bind _returnvalue_2 (`MaterialInstanceDynamic.K2_GetScalarParameterValue` (`self.MaterialInstanceDynamic`) (`self.ValName`)))
  (if (or (or (and (<= _returnvalue_2 0.0) (not _fadein)) (and (>= _returnvalue_2 1.0) _fadein)) (> (`self.GetGameTimeSinceCreation`) 0.5))
    (`self.K2_DestroyActor`)
    (elif (`self.FadeIn`)
      (`MaterialInstanceDynamic.SetScalarParameterValue` _materialinstancedynamic _valname (+ _returnvalue _returnvalue_2))
      (else
        (`MaterialInstanceDynamic.SetScalarParameterValue` _materialinstancedynamic _valname (- _returnvalue_2 _returnvalue))))))

(fn `UserConstructionScript`)