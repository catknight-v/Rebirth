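; BP_DoorTrack_Up is a helper actor that slides its owner, presumably a door, vertically by Distance over Duration.
; BeginPlay caches the owner and its starting location.
; Tick applies a cosine ease-in/out Z offset from that start, timed from the helper's own creation, without sweeping.
; Once Duration has passed, it disables its tick without setting a final position.
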(event `self.ReceiveBeginPlay`
  (bind _output_get (set `self.MoveActor` (`self.GetOwner`)))
  (set `self.PreLocation` (`self.K2_GetActorLocation` _output_get)))

(event `self.ReceiveTick`
  (params (DeltaSeconds :type "Float (single-precision)"))
  (bind _returnvalue (`self.GetGameTimeSinceCreation`))
  (if (> _returnvalue (`self.Duration`))
    (`self.SetActorTickEnabled` false)
    (else
      (`self.K2_SetActorLocation` (`self.MoveActor`) (+ (`KismetMathLibrary.MakeVector` 0.0 0.0 (/ (* (- 1.0 (`KismetMathLibrary.DegCos` (/ (* _returnvalue 180.0) (`self.Duration`)))) (`self.Distance`)) 2.0)) (`self.PreLocation`)) false false))))

(fn `UserConstructionScript`)