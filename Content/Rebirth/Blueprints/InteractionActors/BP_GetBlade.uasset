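; Interactable blade pickup that the player can collect once, with its collected state persisted in the save game.
; BeginPlay reads the PlayerGetWeapon status to show or hide the mesh and toggle box collision.
; Entering or leaving the area fades the prompt widget; interacting gives the combat player controller an item, writes the status to the save, and hides the actor.
; CanInteract always returns false, while Interactwith does not check it.
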(event `self.ReceiveBeginPlay`
  (bind _box (`self.Box`))
  (bind _skeletalmesh (`self.SkeletalMesh`))
  (bind _asbp_rebirth_game_instance (cast `/Game/Rebirth/Blueprints/Rebirth/BP_RebirthGameInstance` (`GameplayStatics.GetGameInstance`)))
  (bind _returnvalue (`RebirthGameInstance.GetCurrentSaveGame` _asbp_rebirth_game_instance))
  (bind _returnvalue_2 (`RebirthSaveGame.StatusInquiry` _returnvalue (`self.PlayerGetWeapon`) 0))
  (if (== _returnvalue_2 0)
    (`PrimitiveComponent.SetCollisionEnabled` _box "QueryOnly")
    (`SceneComponent.SetVisibility` _skeletalmesh true false)
    (else
      (`PrimitiveComponent.SetCollisionEnabled` _box "NoCollision")
      (`SceneComponent.SetVisibility` _skeletalmesh false false))))

(event `InteractionInterface.EnterInteractableArea`
  (params (Interactor :type "Actor Object Reference"))
  (bind _asbp_ewidget (cast `/Game/Rebirth/UI/BP_EWidget` (`WidgetComponent.GetUserWidgetObject` (`self.EWidget`))))
  (`/Game/Rebirth/UI/BP_EWidget.EFadeIn` _asbp_ewidget))

(event `InteractionInterface.LeaveInteractableArea`
  (params (Interactor :type "Actor Object Reference"))
  (bind _asbp_ewidget (cast `/Game/Rebirth/UI/BP_EWidget` (`WidgetComponent.GetUserWidgetObject` (`self.EWidget`))))
  (`/Game/Rebirth/UI/BP_EWidget.EFadeOut` _asbp_ewidget))

(event `InteractionInterface.InteractWith`
  (params (Interactor :type "Actor Object Reference"))
  (bind _asbp_rebirth_combat_pc (cast `/Game/Rebirth/Blueprints/Characters/BP_RebirthCombatPC` Interactor))
  (`RebirthCombatPC.GetItem` _asbp_rebirth_combat_pc "WeaponItem:Blade" 1)
  (bind _asbp_rebirth_game_instance (cast `/Game/Rebirth/Blueprints/Rebirth/BP_RebirthGameInstance` (`GameplayStatics.GetGameInstance`)))
  (bind _returnvalue (`RebirthGameInstance.GetCurrentSaveGame` _asbp_rebirth_game_instance))
  (`RebirthSaveGame.StatusUpdate` _returnvalue (`self.PlayerGetWeapon`) 1)
  (`RebirthGameInstance.WriteSaveGame` _asbp_rebirth_game_instance)
  (`PrimitiveComponent.SetCollisionEnabled` (`self.Box`) "NoCollision")
  (`SceneComponent.SetVisibility` (`self.SkeletalMesh`) false false))

(fn `CanInteract`
  (params (Interactor :type "Actor Object Reference"))
  (returns (ReturnValue :type Boolean))
  (return false))

(fn `UserConstructionScript`)