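; NPCsLive is a level actor that watches two referenced NPCs and advances the game once both are dead.
; Tick polls both IsAlive states, then AllDead disables ticking so it fires only once.
; AllDead async-loads the Map_3_Gameplay streaming level as visible and has the RebirthPlayerController play the TenaciousYou act.
; An unconnected chain for saving the current level to the game instance's save is left unused.
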(event `self.ReceiveTick`
  (params (DeltaSeconds :type "Float (single-precision)"))
  (if (and (not (`RebirthCombatCharacterBase.IsAlive` (`self.NPC1`))) (not (`RebirthCombatCharacterBase.IsAlive` (`self.NPC2`))))
    (`self.AllDead`)))

(event `AllDead`
  (`self.SetActorTickEnabled` false)
  (`GameplayStatics.LoadStreamLevel` "Map_3_Gameplay" true)
  (bind _asrebirth_player_controller (cast `RebirthPlayerController` (`GameplayStatics.GetPlayerController` 0)))
  (`RebirthPlayerController.PlayAnAct` _asrebirth_player_controller "/Game/Rebirth/Acts/Act_TenaciousYou.Act_TenaciousYou_C"))

(fn `UserConstructionScript`)