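; BP_RebirthCombatPC is the player combat character, linking damage, health and death events to HUD and level flow.
; On BeginPlay it creates the attribute widget, which health changes update with the current health ratio.
; Taking damage snaps the character to face the damage causer and sends it an Event.Hit gameplay event.
; Death asks the Rebirth player controller to reset the level.
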(event `self.ReceiveBeginPlay`
  (bind `_as玩家控制器` (cast `PlayerController` (`self.GetController`)))
  (bind _returnvalue (`|CreateWidget` "/Game/Rebirth/UI/BP_PlayerAttributeWidget.BP_PlayerAttributeWidget_C" `_as玩家控制器`))
  (bind _output_get (set `self.AttributeWidget` _returnvalue))
  (`UserWidget.AddToViewport` _output_get 0))

(event `self.OnDamaged`
  (params (DamageAmount :type "Float (single-precision)") (HitInfo :type "HitResult Structure (by ref)") (DamageTags :type "GameplayTagContainer Structure (by ref)") (InstigatorCharacter :type "RebirthCombatCharacterBase Object Reference") (DamageCauser :type "Actor Object Reference"))
  (`self.FaceToInstantly` (`self.K2_GetActorLocation` DamageCauser))
  (`AbilitySystemBlueprintLibrary.SendGameplayEventToActor` self (struct :`TagName` "Event.Hit")))

(event `self.OnDeath`
  (params (DamageAmount :type "Float (single-precision)") (HitInfo :type "HitResult Structure (by ref)") (DamageTags :type "GameplayTagContainer Structure (by ref)") (InstigatorCharacter :type "RebirthCombatCharacterBase Object Reference") (DamageCauser :type "Actor Object Reference"))
  (bind _asbp_rebirth_player_controller (cast `/Game/Rebirth/Blueprints/Controllers/BP_RebirthPlayerController` (`self.GetController`)))
  (`/Game/Rebirth/Blueprints/Controllers/BP_RebirthPlayerController.LevelReset` _asbp_rebirth_player_controller))

(event `self.OnHealthChanged`
  (params (DeltaValue :type "Float (single-precision)") (EventTags :type "GameplayTagContainer Structure (by ref)"))
  (`/Game/Rebirth/UI/BP_PlayerAttributeWidget.HealthSet` (`self.AttributeWidget`) (/ (`self.GetHealth`) (`self.GetMaxHealth`))))

(fn `UserConstructionScript`)