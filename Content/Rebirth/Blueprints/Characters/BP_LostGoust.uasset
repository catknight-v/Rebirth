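; BP_LostGoust is a character Blueprint for the Lost Goust, which fights with a talon weapon actor.
; On BeginPlay it spawns BP_TalonActor as owner and instigator and attaches it to a right-hand middle-finger socket on the mesh.
; When damaged it snaps to face the damage causer and sends itself an Event.Hit gameplay event.
; The talon is destroyed along with the character.
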(event `self.ReceiveBeginPlay`
  (bind _returnvalue (`|SpawnActorFromClass` "/Game/Rebirth/Blueprints/Weapons/BP_TalonActor.BP_TalonActor_C" (`KismetMathLibrary.MakeTransform` (0.0 0.0 0.0)) "Undefined" "OverrideRootScale" self self))
  (bind _output_get (set `self.WeaponTalon` _returnvalue))
  (`self.K2_AttachToComponent` _output_get (`self.Mesh`) "middle_01_r_socket" "KeepRelative" "KeepRelative" "KeepRelative" true))

(event `self.OnDamaged`
  (params (DamageAmount :type "Float (single-precision)") (HitInfo :type "HitResult Structure (by ref)") (DamageTags :type "GameplayTagContainer Structure (by ref)") (InstigatorCharacter :type "RebirthCombatCharacterBase Object Reference") (DamageCauser :type "Actor Object Reference"))
  (`self.FaceToInstantly` (`self.K2_GetActorLocation` DamageCauser))
  (`AbilitySystemBlueprintLibrary.SendGameplayEventToActor` self (struct :`TagName` "Event.Hit")))

(event `self.ReceiveDestroyed`
  (`self.K2_DestroyActor` (`self.WeaponTalon`)))

(fn `UserConstructionScript`)